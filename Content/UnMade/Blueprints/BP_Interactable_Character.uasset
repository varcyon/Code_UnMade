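; Interactable character base that flags its skeletal meshes in the custom depth stencil while the cursor hovers over it.
; GetMeshes caches all skeletal mesh components and enables custom depth rendering on them, though nothing in this graph calls it.
; MouseInteractionBox cursor-over events set the cached meshes' stencil value on enter and reset it to zero on exit.
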(event OnBeginCursorOver(MouseInteractionBox)
  (params (TouchedComponent :type Primitive%20Component%20Object%20Reference))
  (for _array_element (Variables|Default|GetMeshs)
    (Rendering|SetCustomDepthStencilValue _array_element 2)))

(event OnEndCursorOver(MouseInteractionBox)
  (params (TouchedComponent :type Primitive%20Component%20Object%20Reference))
  (for _array_element (Variables|Default|GetMeshs)
    (Rendering|SetCustomDepthStencilValue _array_element 0)))

(event EventBeginPlay)

(event Collision|EventActorBeginOverlap
  (params (OtherActor :type Actor%20Object%20Reference)))

(event EventTick
  (params (DeltaSeconds :type Float%20%28single-precision%29)))

(fn ConstructionScript)

(fn GetMeshes
  (bind _output_get (Variables|Default|SetMeshs (Actor|GetComponentsByClass "/Script/Engine.SkeletalMeshComponent")))
  (for _array_element _output_get
    (Rendering|SetRenderCustomDepth _array_element true)))