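; BP_Damagable_Actor is an actor Blueprint that flags its static meshes on mouse hover; despite the name, it contains no damage logic.
; MouseInteractionBox cursor events toggle the custom depth stencil value on every valid entry in Meshes, likely for a highlight effect.
; GetMeshes fills that array from the actor's static mesh components and enables custom depth rendering, but nothing in this file calls it.
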(event OnBeginCursorOver(MouseInteractionBox)
  (params (TouchedComponent :type Primitive%20Component%20Object%20Reference))
  (for _array_element (Variables|Default|GetMeshes)
    (Utilities|IsValid _array_element
      (:Is%20Valid
        (Rendering|SetCustomDepthStencilValue _array_element 1)))))

(event OnEndCursorOver(MouseInteractionBox)
  (params (TouchedComponent :type Primitive%20Component%20Object%20Reference))
  (for _array_element (Variables|Default|GetMeshes)
    (Utilities|IsValid _array_element
      (:Is%20Valid
        (Rendering|SetCustomDepthStencilValue _array_element 0)))))

(event Collision|EventActorBeginOverlap
  (params (OtherActor :type Actor%20Object%20Reference)))

(event EventTick
  (params (DeltaSeconds :type Float%20%28single-precision%29)))

(fn ConstructionScript)

(fn GetMeshes
  (bind _output_get (Variables|Default|SetMeshes (Actor|GetComponentsByClass "/Script/Engine.StaticMeshComponent")))
  (for _array_element _output_get
    (Rendering|SetRenderCustomDepth _array_element true)))