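; Player character Blueprint that drives XP gain and leveling through the Gameplay Ability System, using GAS Companion's core component.
; Current Exp changes show an XP number and, at the threshold, apply GE_LevelUp with overflow XP as a SetByCaller magnitude.
; XP and level-up widget components spawn locally in standalone, otherwise via multicasts that skip the server.
; Essence, hunger and thirst depletion handlers apply GE_Ablaze but are never called.
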(event OnPostGameplayEffectExecute(GSCCore)
  (params (Attribute :type Gameplay%20Attribute%20Structure) (SourceActor :type Actor%20Object%20Reference) (TargetActor :type Actor%20Object%20Reference) (SourceTags :type Gameplay%20Tag%20Container%20Structure%20%28by%20ref%29) (Payload :type GSC%20Gameplay%20Effect%20Execute%20Data%20Structure))
  (|SwitchGameplayAttribute Attribute
    (:CurrentExp
      (CallFunction|DisplayXPNumber (.deltavalue Payload))
      (CallFunction|HandleXPChange (.deltavalue Payload)))))

(event OnAttributeChange(GSCCore)
  (params (Attribute :type Gameplay%20Attribute%20Structure) (DeltaValue :type Float%20%28single-precision%29) (EventTags :type Gameplay%20Tag%20Container%20Structure))
  (|SwitchGameplayAttribute Attribute
    (:Level
      (CallFunction|ReplicateddAddLevelUPWC))))

(event Custom|ReplicateddAddLevelUPWC
  ;[1 1 1] Showing Level up and on Network
  (if (Class|KismetSystemLibrary|IsStandalone)
    (CallFunction|AddLevelUPWC)
    (else
      (CallFunction|MulticastAddLevelUPWC))))

(event Custom|Multicast_AddXPNumberWC
  (params (Number :type Float%20%28double-precision%29))
  (if (not (Networking|IsServer))
    (CallFunction|AddXPNumberWC Number)))

(event Custom|AddXPNumberWC
  (params (Number :type Float%20%28double-precision%29))
  (bind _returnvalue (AddComponent|AddWCXPText true (Transformation|GetActorTransform)))
  (Default|SetNumber _returnvalue Number))

(event Custom|ReplicatedAddXPNumberWC
  (params (Number :type Float%20%28double-precision%29))
  (if (Class|KismetSystemLibrary|IsStandalone)
    (CallFunction|AddXPNumberWC Number)
    (else
      (CallFunction|MulticastAddXPNumberWC Number))))

(event Custom|AddLevelUPWC
  ;[1 1 1] Showing Level up and on Network
  (bind _returnvalue (AddComponent|AddWCLevelUp true (Transformation|GetActorTransform)))
  (Default|SetNumber _returnvalue 0.0))

(event Custom|Multicast_AddLevelUPWC
  ;[1 1 1] Showing Level up and on Network
  (if (not (Networking|IsServer))
    (CallFunction|AddLevelUPWC)))

(event EventBeginPlay
  (bind _gsccore (Variables|Default|GetGSCCore))
  (Development|PrintText (Utilities|Text|FormatText "{Level} : {C} :{N} " (Class|GSCCoreComponent|GetAttributeValue _gsccore "(AttributeName=\"Essence\",Attribute=/Script/Code_UnMade.SurvivalAttributeSet:Essence,AttributeOwner=None)") (Class|GSCCoreComponent|GetAttributeValue _gsccore "(AttributeName=\"Hungry\",Attribute=/Script/Code_UnMade.SurvivalAttributeSet:Hungry,AttributeOwner=None)") (Class|GSCCoreComponent|GetAttributeValue _gsccore "(AttributeName=\"Thirst\",Attribute=/Script/Code_UnMade.SurvivalAttributeSet:Thirst,AttributeOwner=None)"))))

(fn ConstructionScript
  (|CallParentFunction))

(fn HandleXPChange
  (params (Delta%20Value :type Float%20%28double-precision%29))
  (bind _gsccore (Variables|Default|GetGSCCore))
  (LocalVariables|SetCurrentXp (Class|GSCCoreComponent|GetAttributeValue _gsccore "(AttributeName=\"CurrentExp\",Attribute=/Script/Code_UnMade.ExperienceAttributeSet:CurrentExp,AttributeOwner=/Script/CoreUObject.Class'\"/Script/Code_UnMade.ExperienceAttributeSet\"')"))
  (LocalVariables|SetNextLevelXP (Class|GSCCoreComponent|GetAttributeValue _gsccore "(AttributeName=\"NeededExp\",Attribute=/Script/Code_UnMade.ExperienceAttributeSet:NeededExp,AttributeOwner=/Script/CoreUObject.Class'\"/Script/Code_UnMade.ExperienceAttributeSet\"')"))
  (Development|PrintString (Utilities|String|ToString(Text) (Utilities|Text|FormatText "{Level} : {c} : {n}" (Class|GSCCoreComponent|GetAttributeValue _gsccore "(AttributeName=\"Level\",Attribute=/Script/Code_UnMade.ExperienceAttributeSet:Level,AttributeOwner=/Script/CoreUObject.Class'\"/Script/Code_UnMade.ExperienceAttributeSet\"')") (LocalVariables|GetCurrentXp) (LocalVariables|GetNextLevelXP))))
  (if (>= (LocalVariables|GetCurrentXp) (LocalVariables|GetNextLevelXP))
    (bind _returnvalue (Ability|GameplayEffect|AssignTagSetbyCallerMagnitude (GameplayEffects|MakeOutgoingSpec :self (Variables|Default|GetAbilitySystemComponent) :GameplayEffectClass "/Game/UnMade/GamePlay_Effects/GE_LevelUp.GE_LevelUp_C" :Level (+ (Class|GSCCoreComponent|GetAttributeValue (Variables|Default|GetGSCCore) "(AttributeName=\"Level\",Attribute=/Script/Code_UnMade.ExperienceAttributeSet:Level,AttributeOwner=/Script/CoreUObject.Class'\"/Script/Code_UnMade.ExperienceAttributeSet\"')") 1.0)) "(TagName=\"SetByCaller.XP.Magnitude\")" (- (LocalVariables|GetCurrentXp) (LocalVariables|GetNextLevelXP))))
    (GameplayEffects|ApplyGameplayEffectSpecToSelf (Variables|Default|GetAbilitySystemComponent) _returnvalue)))

(fn DisplayXPNumber
  (params (Number :type Float%20%28double-precision%29))
  (if (!= Number 0.0)
    (CallFunction|ReplicatedAddXPNumberWC Number)))

(fn HandleEssenceChange
  (params (Delta%20Value :type Float%20%28double-precision%29))
  (LocalVariables|SetCurrentEssence (Class|GSCCoreComponent|GetAttributeValue (Variables|Default|GetGSCCore) "(AttributeName=\"Essence\",Attribute=/Script/Code_UnMade.SurvivalAttributeSet:Essence,AttributeOwner=None)"))
  (if (<= (LocalVariables|GetCurrentEssence) 0.0)
    (GameplayEffects|ApplyGameplayEffectSpecToSelf (Variables|Default|GetAbilitySystemComponent) (GameplayEffects|MakeOutgoingSpec :self (Variables|Default|GetAbilitySystemComponent) :GameplayEffectClass "/Game/UnMade/GamePlay_Effects/Fire/Ablaze/GE_Ablaze.GE_Ablaze_C"))))

(fn HandleHungerChange
  (params (Delta%20Value :type Float%20%28double-precision%29))
  (LocalVariables|SetCurrentHunger (Class|GSCCoreComponent|GetAttributeValue (Variables|Default|GetGSCCore) "(AttributeName=\"Hungry\",Attribute=/Script/Code_UnMade.SurvivalAttributeSet:Hungry,AttributeOwner=None)"))
  (if (<= (LocalVariables|GetCurrentHunger) 0.0)
    (GameplayEffects|ApplyGameplayEffectSpecToSelf (Variables|Default|GetAbilitySystemComponent) (GameplayEffects|MakeOutgoingSpec :self (Variables|Default|GetAbilitySystemComponent) :GameplayEffectClass "/Game/UnMade/GamePlay_Effects/Fire/Ablaze/GE_Ablaze.GE_Ablaze_C"))))

(fn HandleThirstChange
  (params (Delta%20Value :type Float%20%28double-precision%29))
  (LocalVariables|SetCurrentThirst (Class|GSCCoreComponent|GetAttributeValue (Variables|Default|GetGSCCore) "(AttributeName=\"Thirst\",Attribute=/Script/Code_UnMade.SurvivalAttributeSet:Thirst,AttributeOwner=None)"))
  (if (<= (LocalVariables|GetCurrentThirst) 0.0)
    (GameplayEffects|ApplyGameplayEffectSpecToSelf (Variables|Default|GetAbilitySystemComponent) (GameplayEffects|MakeOutgoingSpec :self (Variables|Default|GetAbilitySystemComponent) :GameplayEffectClass "/Game/UnMade/GamePlay_Effects/Fire/Ablaze/GE_Ablaze.GE_Ablaze_C"))))