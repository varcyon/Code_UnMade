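; Player state Blueprint for UnMade that grants the player character its slotted Gameplay Ability System abilities.
; On BeginPlay it casts player 0's character to BP_PlayerCharacter, caches it and its Ability System Component, then gives each SlottedAbilities entry at level 1, using the array index as InputID.
; CalculateLifeForceMaxCarry is an empty stub, and Tick does nothing.
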(event EventBeginPlay
  (bind _asbp_player_character (Utilities|Casting|CastToBP_PlayerCharacter (Game|GetPlayerCharacter 0)))
  (Variables|Default|SetAs%20BP%20Player%20Character _asbp_player_character)
  (Variables|Default|SetASC (Ability|GetAbilitySystemComponent _asbp_player_character))
  (for (_array_element _array_index) (Variables|Default|GetSlottedAbilities)
    (GameplayAbilities|GiveAbility (Variables|Default|GetASC) _array_element 1 _array_index))
  (Development|PrintString "Slotted Abilities Given"))

(event EventTick
  (params (DeltaSeconds :type Float%20%28single-precision%29)))

(fn ConstructionScript)

(fn CalculateLifeForceMaxCarry)